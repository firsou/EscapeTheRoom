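; Openable door actor that swings open and shut when its OpenDoor events fire.
; BeginPlay caches the starting rotation, and the DoorAnim timeline adds its OpenAngle yaw to that rotation each update.
; OnOpen plays the timeline and OnClose reverses it.
; A timeline event track plays the Doorclose sound at the door's location.
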(event OnOpen(OpenDoor)
  (bind _openangle (Timeline|DoorAnim Play)
    (:Update
      (Transformation|SetActorRotation (Math|Rotator|CombineRotators (Math|Rotator|MakeRotator 0.0 0.0 _openangle) (Variables|Default|GetBeginRotation))))
    (:PlaySound
      (Audio|PlaySoundatLocation "/Game/doorclose.doorclose" (Transformation|GetActorLocation)))))

(event OnClose(OpenDoor)
  (bind _openangle (Timeline|DoorAnim Reverse)
    (:Update
      (Transformation|SetActorRotation (Math|Rotator|CombineRotators (Math|Rotator|MakeRotator 0.0 0.0 _openangle) (Variables|Default|GetBeginRotation))))
    (:PlaySound
      (Audio|PlaySoundatLocation "/Game/doorclose.doorclose" (Transformation|GetActorLocation)))))

(event EventBeginPlay
  (Variables|Default|SetBeginRotation (Transformation|GetActorRotation)))

(fn ConstructionScript)